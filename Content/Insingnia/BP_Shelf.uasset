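; BP_Shelf is a display shelf that shows the player's unlocked insignias as meshes.
; On BeginPlay it caches GI_MyGameInstance and binds to its insignia-unlocked event.
; Each unlock re-queries insignias by state and spawns a static mesh component at each shelf socket in order, stopping at the first invalid entry.
; Earlier components are not cleared, so repeated unlocks stack duplicates; a debug string prints per placed mesh.
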(event Custom|OnInsigniaUnlocked
  (params (PDA%20Insignia :type PDA%20Insignia%20Object%20Reference))
  (bind _shelf (Variables|Default|GetShelf))
  (bind _unlockedinsignias (Default|GetInsigniasbyState (Variables|Default|GetGI%20My%20Game%20Instance) "NewEnumerator1"))
  (Variables|Default|SetUnlocked%20Insignias _unlockedinsignias)
  (bind (_array_element _array_index) (Utilities|Array|ForEachLoopwithBreak (Transformation|GetAllSocketNames _shelf) :!label _label)
    (:LoopBody
      (Utilities|IsValid (Utilities|Array|Get(acopy) (Variables|Default|GetUnlocked%20Insignias) _array_index)
        (:Is%20Valid
          (bind _returnvalue (AddComponent|AddStaticMeshComponent false (Transformation|GetSocketTransform _shelf _array_element "RTS_Actor")))
          (Components|StaticMesh|SetStaticMesh _returnvalue (.insigniamesh (Variables|/Game/Insingnia/Data/PDA_Insignia.PDA_Insignia_C|GetInsignia (Utilities|Array|Get(acopy) (Variables|Default|GetUnlocked%20Insignias) _array_index))))
          (Development|PrintString "DESBLOQUEADO" true true "(R=0.000000,G=0.660000,B=1.000000,A=1.000000)" 1e+01))
        (:Is%20Not%20Valid
          (goto _label Break))))))

(event EventBeginPlay
  (Utilities|FlowControl|Sequence
    (:then_0
      (bind _asgi_my_game_instance (Utilities|Casting|CastToGI_MyGameInstance (Game|GetGameInstance)))
      (Variables|Default|SetGI%20My%20Game%20Instance _asgi_my_game_instance))
    (:then_1
      (EventDispatchers|BindEventtoOnInsigniaUnlocked (Variables|Default|GetGI%20My%20Game%20Instance) (delegate Custom|OnInsigniaUnlocked)))))

(fn ConstructionScript)
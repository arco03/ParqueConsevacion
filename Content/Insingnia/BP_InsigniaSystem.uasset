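; BP_InsigniaSystem is a Blueprint that tracks insignias and awards the Zone 1 insignia when its sphere is overlapped.
; The overlap passes a hardcoded DA_InsigniaZona1 to GiveInsignia, without filtering the overlapping actor.
; GiveInsignia finds the InsigniaList entry with a matching name, changes its state enum, prints that state on screen and stops searching.
; ShowInsignia is an empty stub.
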(event OnComponentBeginOverlap(Sphere)
  (params (OverlappedComponent :type Primitive%20Component%20Object%20Reference) (OtherActor :type Actor%20Object%20Reference) (OtherComp :type Primitive%20Component%20Object%20Reference) (OtherBodyIndex :type Integer) (bFromSweep :type Boolean) (SweepResult :type Hit%20Result%20Structure%20%28by%20ref%29))
  (CallFunction|GiveInsignia "/Game/Insingnia/Data/DA_InsigniaZona1.DA_InsigniaZona1"))

(fn ConstructionScript)

(fn ShowInsignia)

(fn GiveInsignia
  (params (Insignia :type PDA%20Insignia%20Object%20Reference))
  (bind _insignialist (Variables|Default|GetInsigniaList))
  (bind (_array_element _array_index) (Utilities|Array|ForEachLoopwithBreak _insignialist :!label _label)
    (:LoopBody
      (if (Utilities|Enum|Equal(Enum) (.insignianame (Variables|/Game/Insingnia/Data/PDA_Insignia.PDA_Insignia_C|GetInsignia Insignia)) (.insignianame (Variables|/Game/Insingnia/Data/PDA_Insignia.PDA_Insignia_C|GetInsignia (.insigniadata _array_element))))
        (Utilities|FlowControl|Sequence
          (:then_0
            (bind _structout (Utilities|Struct|SetmembersinF_InsigniaState (Utilities|Array|Get(acopy) _insignialist _array_index) "NewEnumerator1"))
            (Development|PrintString (Utilities|String|EnumtoString (.insigniastate _structout)) true true "(R=1.000000,G=0.953341,B=0.000000,A=1.000000)" 2e+01))
          (:then_1
            (goto _label Break)))))))
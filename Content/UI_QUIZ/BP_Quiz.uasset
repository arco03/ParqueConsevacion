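; VR quiz station actor that shows a question on a world widget and takes answers through four physical buttons.
; When the VRPawn enters the main box, it loads a row from the Questions DataTable into DP_Widget2, along with an Insignia.
; Each button's overlap box animates its button along Z using the shared ButtonMoveOn helper and MoveComponentTo.
; Beginning an overlap also sends that button's answer index to the widget.
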(event OnComponentBeginOverlap(Box3)
  (params (OverlappedComponent :type Primitive%20Component%20Object%20Reference) (OtherActor :type Actor%20Object%20Reference) (OtherComp :type Primitive%20Component%20Object%20Reference) (OtherBodyIndex :type Integer) (bFromSweep :type Boolean) (SweepResult :type Hit%20Result%20Structure%20%28by%20ref%29))
  ;[0.15 0.15 0.15 0.5] ButtonC
  (bind (_finalpositionmove _buttonfinal _finalposition) (CallFunction|ButtonMoveon (Variables|Default|GetPressButton2) OtherActor))
  (Components|MoveComponentTo _buttonfinal (Math|Vector|MakeVector 0.0 0.0 _finalposition) "0, 0, 0" false false 0.2 false)
  (Default|Answer (Variables|Default|GetAs%20DP%20Widget%202) 2))

(event OnComponentEndOverlap(Box3)
  (params (OverlappedComponent :type Primitive%20Component%20Object%20Reference) (OtherActor :type Actor%20Object%20Reference) (OtherComp :type Primitive%20Component%20Object%20Reference) (OtherBodyIndex :type Integer))
  ;[0.15 0.15 0.15 0.5] ButtonC
  (bind (_finalpositionmove _buttonfinal) (CallFunction|ButtonMoveon (Variables|Default|GetPressButton2) OtherActor))
  (Components|MoveComponentTo _buttonfinal (Math|Vector|MakeVector 0.0 0.0 _finalpositionmove) "0, 0, 0" false false 0.2 false))

(event OnComponentBeginOverlap(Box)
  (params (OverlappedComponent :type Primitive%20Component%20Object%20Reference) (OtherActor :type Actor%20Object%20Reference) (OtherComp :type Primitive%20Component%20Object%20Reference) (OtherBodyIndex :type Integer) (bFromSweep :type Boolean) (SweepResult :type Hit%20Result%20Structure%20%28by%20ref%29))
  (Utilities|Casting|CastToVRPawn OtherActor)
  (bind _returnvalue (Utilities|GetDataTableRow (Variables|Default|GetQuestions) (Variables|Default|GetrowName))
    (:then
      (Default|FillQuizz (Variables|Default|GetAs%20DP%20Widget%202) _returnvalue (Variables|Default|GetInsignia)))
    (:RowNotFound
      (Development|PrintString "Row NO encontrada"))))

(event OnComponentBeginOverlap(Box1)
  (params (OverlappedComponent :type Primitive%20Component%20Object%20Reference) (OtherActor :type Actor%20Object%20Reference) (OtherComp :type Primitive%20Component%20Object%20Reference) (OtherBodyIndex :type Integer) (bFromSweep :type Boolean) (SweepResult :type Hit%20Result%20Structure%20%28by%20ref%29))
  ;[0.15 0.15 0.15 0.5] ButtonA
  (bind (_finalpositionmove _buttonfinal _finalposition) (CallFunction|ButtonMoveon (Variables|Default|GetPressButton) OtherActor))
  (Components|MoveComponentTo _buttonfinal (Math|Vector|MakeVector 0.0 0.0 _finalposition) "0, 0, 0" false false 0.2 false)
  (Default|Answer (Variables|Default|GetAs%20DP%20Widget%202)))

(event OnComponentEndOverlap(Box1)
  (params (OverlappedComponent :type Primitive%20Component%20Object%20Reference) (OtherActor :type Actor%20Object%20Reference) (OtherComp :type Primitive%20Component%20Object%20Reference) (OtherBodyIndex :type Integer))
  ;[0.15 0.15 0.15 0.5] ButtonA
  (bind (_finalpositionmove _buttonfinal) (CallFunction|ButtonMoveon (Variables|Default|GetPressButton) OtherActor))
  (Components|MoveComponentTo _buttonfinal (Math|Vector|MakeVector 0.0 0.0 _finalpositionmove) "0, 0, 0" false false 0.2 false))

(event OnComponentBeginOverlap(Box2)
  (params (OverlappedComponent :type Primitive%20Component%20Object%20Reference) (OtherActor :type Actor%20Object%20Reference) (OtherComp :type Primitive%20Component%20Object%20Reference) (OtherBodyIndex :type Integer) (bFromSweep :type Boolean) (SweepResult :type Hit%20Result%20Structure%20%28by%20ref%29))
  ;[0.15 0.15 0.15 0.5] ButtonA
  (bind (_finalpositionmove _buttonfinal _finalposition) (CallFunction|ButtonMoveon (Variables|Default|GetPressButton1) OtherActor))
  (Components|MoveComponentTo _buttonfinal (Math|Vector|MakeVector 0.0 0.0 _finalposition) "0, 0, 0" false false 0.2 false)
  (Default|Answer (Variables|Default|GetAs%20DP%20Widget%202) 1))

(event OnComponentEndOverlap(Box2)
  (params (OverlappedComponent :type Primitive%20Component%20Object%20Reference) (OtherActor :type Actor%20Object%20Reference) (OtherComp :type Primitive%20Component%20Object%20Reference) (OtherBodyIndex :type Integer))
  ;[0.15 0.15 0.15 0.5] ButtonA
  (bind (_finalpositionmove _buttonfinal) (CallFunction|ButtonMoveon (Variables|Default|GetPressButton1) OtherActor))
  (Components|MoveComponentTo _buttonfinal (Math|Vector|MakeVector 0.0 0.0 _finalpositionmove) "0, 0, 0" false false 0.2 false))

(event OnComponentBeginOverlap(Box4)
  (params (OverlappedComponent :type Primitive%20Component%20Object%20Reference) (OtherActor :type Actor%20Object%20Reference) (OtherComp :type Primitive%20Component%20Object%20Reference) (OtherBodyIndex :type Integer) (bFromSweep :type Boolean) (SweepResult :type Hit%20Result%20Structure%20%28by%20ref%29))
  ;[0.15 0.15 0.15 0.5] ButtonD
  (bind (_finalpositionmove _buttonfinal _finalposition) (CallFunction|ButtonMoveon (Variables|Default|GetPressButton3) OtherActor))
  (Components|MoveComponentTo _buttonfinal (Math|Vector|MakeVector 0.0 0.0 _finalposition) "0, 0, 0" false false 0.2 false)
  (Default|Answer (Variables|Default|GetAs%20DP%20Widget%202) 3))

(event OnComponentEndOverlap(Box4)
  (params (OverlappedComponent :type Primitive%20Component%20Object%20Reference) (OtherActor :type Actor%20Object%20Reference) (OtherComp :type Primitive%20Component%20Object%20Reference) (OtherBodyIndex :type Integer))
  ;[0.15 0.15 0.15 0.5] ButtonD
  (bind (_finalpositionmove _buttonfinal) (CallFunction|ButtonMoveon (Variables|Default|GetPressButton3) OtherActor))
  (Components|MoveComponentTo _buttonfinal (Math|Vector|MakeVector 0.0 0.0 _finalpositionmove) "0, 0, 0" false false 0.2 false))

(event OnComponentEndOverlap(Box)
  (params (OverlappedComponent :type Primitive%20Component%20Object%20Reference) (OtherActor :type Actor%20Object%20Reference) (OtherComp :type Primitive%20Component%20Object%20Reference) (OtherBodyIndex :type Integer))
  (Utilities|Casting|CastToVRPawn OtherActor)
  (Rendering|SetVisibility (Variables|Default|GetWidget1) true false))

(event EventBeginPlay
  (Utilities|FlowControl|Sequence
    (:then_0
      (bind _asdp_widget_2 (Utilities|Casting|CastToDP_Widget2 (UserInterface|GetWidget (Variables|Default|GetWidget1))))
      (Variables|Default|SetAs%20DP%20Widget%202 _asdp_widget_2))))

(fn ConstructionScript)

(fn ButtonMoveon
  (params (Button :type Static%20Mesh%20Component%20Object%20Reference) (Collision :type Actor%20Object%20Reference))
  (Utilities|FlowControl|Sequence
    (:then_0
      (Utilities|Casting|CastToVRPawn Collision))
    (:then_1
      (Variables|Default|SetButtonStartPosition (Variables|/Script/Engine.SceneComponent|GetRelativeLocation Button))))
  (return (- (.z (Variables|Default|GetButtonStartPosition)) 5.0) Button (.z (Variables|Default|GetButtonStartPosition))))